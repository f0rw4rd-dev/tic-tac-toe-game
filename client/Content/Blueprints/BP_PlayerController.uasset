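; Player controller for online tic-tac-toe, syncing the board with a REST server through VaRest.
; A Delay on Tick polls about once per second for cleanup and board state, updating the HUD, spawning missing crosses and circles, or returning to Menu on failure.
; Left click posts the current cell as a move and spawns the player's piece.
; Restart requests follow finished games and every board poll, reloading Board on success.
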(event Custom|Restart%20Game%20Send%20Request
  (bind _gameinstance (Variables|Default|GetGameInstance))
  ;[0 0 0] Restart Game
  (bind (_url _varestjson) (CallFunction|InitJsonObjectandURL (Utilities|Text|FormatText "/games/restart?game_id={game_id}&username={username}" (Variables|/Game/Blueprints/BP_GameInstance.BP_GameInstance_C|GetGameId _gameinstance) (Variables|/Game/Blueprints/BP_GameInstance.BP_GameInstance_C|GetUserName _gameinstance)) (Utilities|Map|MakeMap "" "") (Utilities|Map|MakeMap "" 0)))
  (Class|VaRestSubsystem|CallURL (|VaRestSubsystem) _url "POST" "json" _varestjson (delegate Custom|Restart%20Game%20Handle%20Response)))

(event Custom|Get%20Board%20Handle%20Response
  (params (Request :type Va%20Rest%20Request%20JSON%20Object%20Reference))
  ;[0 0 0] Get Board
  (if (== (Class|VaRestRequestJSON|GetResponseCode Request) 200)
    (bind (_success _varestrequest _varestjson) (CallFunction|DecodeResponse Request))
    (if _success
      (Utilities|FlowControl|Sequence
        (:then_0
          (Default|UpdateTurn (Variables|Default|GetHUD) (Class|VaRestJsonObject|GetStringField _varestjson "turn")))
        (:then_1
          (Default|UpdateSide (Variables|Default|GetHUD) (Class|VaRestJsonObject|GetStringField _varestjson "side")))
        (:then_2
          (Default|UpdateStat (Variables|Default|GetHUD) (Class|VaRestJsonObject|GetIntegerField _varestjson "victories.X") (Class|VaRestJsonObject|GetIntegerField _varestjson "victories.O") (Class|VaRestJsonObject|GetIntegerField _varestjson "draws")))
        (:then_3
          (Default|UpdatePlayers (Variables|Default|GetHUD) (Class|VaRestJsonObject|GetIntegerField _varestjson "num_players")))
        (:then_4
          (for _index (range 0 8)
            (if (not (Utilities|Array|Get(acopy) (Variables|Default|GetOccupiedCells) _index))
              (if (not (Utilities|Array|IsEmpty (Class|VaRestJsonObject|GetStringField _varestjson (Utilities|String|ToString(Integer) _index))))
                (bind _asactor (Utilities|Casting|CastToActorClass (Class|KismetMathLibrary|SelectClass "/Game/Blueprints/BP_Cross.BP_Cross_C" "/Game/Blueprints/BP_Circle.BP_Circle_C" (Utilities|Enum|Equal(Enum) (Class|VaRestJsonObject|GetStringField _varestjson (Utilities|String|ToString(Integer) _index)) "X"))))
                (Game|SpawnActorfromClass _asactor (Math|Transform|MakeTransform (Utilities|Array|Get(acopy) (Variables|Default|GetCellLocation) _index) "0, 0, 0" "1.000000,1.000000,1.000000") "Undefined" "MultiplyWithRoot" 0 0)
                (Utilities|Array|SetArrayElem (Variables|Default|GetOccupiedCells) _index true)))))
        (:then_5
          (CallFunction|RestartGameSendRequest))))
    (else
      (Game|OpenLevel(byName) "Menu"))))

(event Custom|Make%20Move%20Send%20Request
  (bind _gameinstance (Variables|Default|GetGameInstance))
  (bind _currentcellnumber (Variables|Default|GetCurrentCellNumber))
  (bind _returnvalue (/ _currentcellnumber 3))
  ;[0 0 0] Make Move
  (if (>= (Variables|Default|GetCurrentCellNumber) 0)
    (bind (_url _varestjson) (CallFunction|InitJsonObjectandURL (Utilities|Text|FormatText "/games/move?game_id={game_id}&username={username}&x={x}&y={y}" (Variables|/Game/Blueprints/BP_GameInstance.BP_GameInstance_C|GetGameId _gameinstance) (Variables|/Game/Blueprints/BP_GameInstance.BP_GameInstance_C|GetUserName _gameinstance) _returnvalue (- (Variables|Default|GetCurrentCellNumber) (* _returnvalue 3))) (Utilities|Map|MakeMap "" "") (Utilities|Map|MakeMap "" 0)))
    (Class|VaRestSubsystem|CallURL (|VaRestSubsystem) _url "POST" "json" _varestjson (delegate Custom|Make%20Move%20Handle%20Response))))

(event Custom|Cleanup%20Handle%20Response
  (params (Request :type Va%20Rest%20Request%20JSON%20Object%20Reference))
  ;[0 0 0] Cleanup
)

(event Custom|Cleanup%20Send%20Request
  ;[0 0 0] Cleanup
  (bind (_url _varestjson) (CallFunction|InitJsonObjectandURL (Utilities|Text|FormatText "/cleanup") (Utilities|Map|MakeMap "" "") (Utilities|Map|MakeMap "" 0)))
  (Class|VaRestSubsystem|CallURL (|VaRestSubsystem) _url "GET" "json" _varestjson (delegate Custom|Cleanup%20Handle%20Response)))

(event Custom|Restart%20Game%20Handle%20Response
  (params (Request :type Va%20Rest%20Request%20JSON%20Object%20Reference))
  ;[0 0 0] Restart Game
  (if (== (Class|VaRestRequestJSON|GetResponseCode Request) 200)
    (bind (_success _varestrequest _varestjson) (CallFunction|DecodeResponse Request))
    (if _success
      (bind _output_get (Variables|/Game/Blueprints/BP_GameInstance.BP_GameInstance_C|SetSide (Variables|Default|GetGameInstance) (Class|VaRestJsonObject|GetStringField _varestjson "side")))
      (bind _asactor (Utilities|Casting|CastToActorClass (Class|KismetMathLibrary|SelectClass "/Game/Blueprints/BP_Cross.BP_Cross_C" "/Game/Blueprints/BP_Circle.BP_Circle_C" (Utilities|Enum|Equal(Enum) _output_get "X"))))
      (Variables|/Game/Blueprints/BP_GameInstance.BP_GameInstance_C|SetActorSide (Variables|Default|GetGameInstance) _asactor)
      (Game|OpenLevel(byName) "Board"))))

(event Custom|Get%20Board%20Send%20Request
  (bind _gameinstance (Variables|Default|GetGameInstance))
  (bind _gameinstance_2 (Variables|Default|GetGameInstance))
  (bind _username (Variables|/Game/Blueprints/BP_GameInstance.BP_GameInstance_C|GetUserName _gameinstance))
  (bind _gameid (Variables|/Game/Blueprints/BP_GameInstance.BP_GameInstance_C|GetGameId _gameinstance_2))
  ;[0 0 0] Get Board
  (Utilities|IsValid (Variables|Default|GetGameInstance)
    (:Is%20Valid
      (if (and (not (Utilities|Array|IsEmpty _gameid)) (not (Utilities|Array|IsEmpty _username)))
        (bind (_url _varestjson) (CallFunction|InitJsonObjectandURL (Utilities|Text|FormatText "/games/{GameId}/{Username}/board" _gameid _username) (Utilities|Map|MakeMap "" "") (Utilities|Map|MakeMap "" 0)))
        (Class|VaRestSubsystem|CallURL (|VaRestSubsystem) _url "GET" "json" _varestjson (delegate Custom|Get%20Board%20Handle%20Response))))))

(event Custom|Make%20Move%20Handle%20Response
  (params (Request :type Va%20Rest%20Request%20JSON%20Object%20Reference))
  ;[0 0 0] Make Move
  (if (== (Class|VaRestRequestJSON|GetResponseCode Request) 200)
    (bind (_success _varestrequest _varestjson) (CallFunction|DecodeResponse Request))
    (if _success
      (Game|SpawnActorfromClass (Variables|/Game/Blueprints/BP_GameInstance.BP_GameInstance_C|GetActorSide (Variables|Default|GetGameInstance)) (Math|Transform|MakeTransform (Utilities|Array|Get(acopy) (Variables|Default|GetCellLocation) (Variables|Default|GetCurrentCellNumber)) "0, 0, 0" "1.000000,1.000000,1.000000") "Undefined" "MultiplyWithRoot" 0 0)
      (Utilities|Array|SetArrayElem (Variables|Default|GetOccupiedCells) (Variables|Default|GetCurrentCellNumber) true)
      (switch int (Class|VaRestJsonObject|GetIntegerField _varestjson "status")
        (:1
          _)
        (:2
          _))
      (CallFunction|RestartGameSendRequest))))

(event EventBeginPlay
  ;[0 0 0] Begin Play
  (bind _asbp_game_instance (Utilities|Casting|CastToBP_GameInstance (Game|GetGameInstance)))
  (Variables|Default|SetGameInstance _asbp_game_instance)
  (if (Variables|Default|GetConnected)
    (CallFunction|GetBoardSendRequest)))

(event EventTick
  (params (DeltaSeconds :type Float%20%28single-precision%29))
  ;[0 0 0] Event Tick
  (Utilities|FlowControl|Delay 1.0)
  (CallFunction|CleanupSendRequest)
  (if (Variables|Default|GetConnected)
    (CallFunction|GetBoardSendRequest)))

(event Input|MouseEvents|LeftMouseButton
  (params (Key :type Key%20Structure :default "None"))
  ;[0 0 0] Make Move
  (:Pressed
    (CallFunction|MakeMoveSendRequest)))

(fn ConstructionScript)

(fn InitJsonObjectandURL
  (params (Params :type Text) (StringFields :type Map%20of%20Strings%20to%20Strings) (Int32Fields :type Map%20of%20Strings%20to%20Integers))
  (bind _returnvalue (Class|VaRestSubsystem|ConstructVaRestJsonObject (|VaRestSubsystem)))
  (bind _output_get (LocalVariables|SetJsonObject _returnvalue))
  (Class|VaRestJsonObject|SetMapFieldsString _output_get StringFields)
  (Class|VaRestJsonObject|SetMapFieldsInt32 (LocalVariables|GetJsonObject) Int32Fields)
  (bind _returnvalue_2 (Utilities|GetDataTableRow "/Game/Configs/DT_Config.DT_Config" "ServerURL")
    (:then
      (return (Utilities|String|ToString(Text) (Utilities|Text|FormatText "{URL}{Params}" (Utilities|Text|ToText(String) (.value _returnvalue_2)) Params)) (LocalVariables|GetJsonObject)))))

(fn DecodeResponse
  (params (Request :type Va%20Rest%20Request%20JSON%20Object%20Reference))
  (bind _returnvalue (Class|VaRestSubsystem|ConstructVaRestJsonObject (|VaRestSubsystem)))
  (LocalVariables|SetJsonObject _returnvalue)
  (bind _returnvalue_2 (Class|VaRestRequestJSON|GetResponseContentasString Request true))
  (bind _returnvalue_3 (Class|VaRestJsonObject|DecodeJson (LocalVariables|GetJsonObject) _returnvalue_2 true))
  (return _returnvalue_3 Request (LocalVariables|GetJsonObject)))